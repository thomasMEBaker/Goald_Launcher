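; Motion controller laser pointer for the launcher's widgets, using the Widget Interaction hit result instead of a line trace.
; Each tick, a blocking hit moves spline point 1 to the hit location and starts the LauncherPawn's timer; otherwise the point stays put and the timer clears.
; UpdateSplineMesh then sets both mesh ends from spline point 1, leaving point 0 unused.
; Per-hand pointer index setup is present but unconnected.
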(event EventBeginPlay
  (bind _aslauncher_pawn (Utilities|Casting|CastToLauncherPawn (Game|Player|GetPlayerPawn 0)))
  (Variables|Default|SetAs%20Launcher%20Pawn _aslauncher_pawn))

(event EventTick
  (params (DeltaSeconds :type Float%20%28single-precision%29))
  (bind _as_launcher_pawn (Variables|Default|GetAs%20Launcher%20Pawn))
  (bind _widgetinteraction (Variables|Default|GetWidgetInteraction))
  (bind _returnvalue (Class|WidgetInteractionComponent|GetLastHitResult _widgetinteraction))
  (bind (_bblockinghit _binitialoverlap _time _distance _location) (Collision|BreakHitResult _returnvalue))
  ;[1 1 1] Use the Hit Result from the Widget Interaction instead of line tracing
  (if _bblockinghit
    ;[1 1 1] Update spline point 1 location
    (Spline|SetLocationatSplinePoint (Variables|Default|GetSpline) 1 _location "World" true)
    ;[1 1 1] Update the spline mesh
    (CallFunction|UpdateSplineMesh)
    (Default|StartTimer _as_launcher_pawn)
    (else
      (Spline|SetLocationatSplinePoint (Variables|Default|GetSpline) 1 (Spline|GetLocationatSplinePoint (Variables|Default|GetSpline) 1 "World") "World" true)
      (CallFunction|UpdateSplineMesh)
      (Default|ClearTimer _as_launcher_pawn))))

(fn ConstructionScript)

(fn UpdateSplineMesh
  (bind _spline (Variables|Default|GetSpline))
  (bind _returnvalue (Spline|GetLocationatSplinePoint _spline 1 "Local"))
  (bind _returnvalue_2 (Spline|GetTangentatSplinePoint _spline 1 "Local"))
  (SplineMesh|SetStartandEnd (Variables|Default|GetSplineMesh) _returnvalue _returnvalue_2 _returnvalue _returnvalue_2 true :!class /Script/Engine.SplineMeshComponent))